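; BP_Project-D sets up the playable scene at BeginPlay, spawning player characters, a cursor actor and the game UI.
; It spawns a character at each PlayerStart, choosing its class from the BP_NeomArenaInstance CharacterType array by index, with BP_Ib mapped to IbTreasureHunter.
; The first player controller possesses the first spawned character, then the cursor spawns at the origin and WBP_UI is added to the viewport.
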(event EventBeginPlay
  (bind _returnvalue (Game|GetPlayerController 0))
  (Utilities|IsValid _returnvalue
    (:Is%20Valid
      (bind _players (CallFunction|SpawnPlayerCharacters (Game|GetGameInstance) (CallFunction|GetCharacterStartPosition)))
      (bind _output_get (Variables|Default|SetPlayers _players))
      (Pawn|Possess _returnvalue (Utilities|Array|Get(acopy) _output_get))
      (bind _cursur (CallFunction|SpawnCursur))
      (Variables|Default|SetCursur _cursur)
      (bind _returnvalue_2 (UserInterface|CreateWidget "/Game/UI/WBP_UI.WBP_UI_C" _returnvalue))
      (bind _output_get_2 (Variables|Default|SetGameUI _returnvalue_2))
      (UserInterface|Viewport|AddtoViewport _output_get_2 0))))

(event EventTick
  (params (DeltaSeconds :type Float%20%28single-precision%29)))

(fn ConstructionScript)

(fn GetCharacterStartPosition
  (bind _position (LocalVariables|GetPosition))
  (bind _outactors (Actor|GetAllActorsOfClass "/Script/Engine.PlayerStart"))
  (for _array_element _outactors
    (Utilities|IsValid _array_element
      (:Is%20Valid
        (Utilities|Array|Add _position (Transformation|GetActorTransform _array_element)))))
  (return _position))

(fn SpawnPlayerCharacters
  (params (GameInstance :type Game%20Instance%20Object%20Reference) (CharacterStartPos :type Array%20of%20Transforms))
  (bind _asbp_neom_arena_instance (Utilities|Casting|CastToBP_NeomArenaInstance GameInstance))
  (Utilities|IsValid _asbp_neom_arena_instance
    (:Is%20Valid
      (for (_array_element _array_index) CharacterStartPos
        (bind _returnvalue (Game|SpawnActorfromClass (Utilities|Select :Index (Utilities|Array|Get(acopy) (Variables|/Game/Blueprints/BP_NeomArenaInstance.BP_NeomArenaInstance_C|GetCharacterType _asbp_neom_arena_instance) _array_index) :NewEnumerator0 "/Game/Characters/BP_Ib.BP_Ib_C") _array_element "Undefined" "MultiplyWithRoot" 0 0))
        (Utilities|Array|Add (LocalVariables|Get__Local_Players) _returnvalue))
      (return (LocalVariables|Get__Local_Players)))))

(fn SpawnCursur
  (bind _returnvalue (Game|SpawnActorfromClass "/Game/UI/BP_Cursur.BP_Cursur_C" (Math|Transform|MakeTransform "0, 0, 0") "Undefined" "MultiplyWithRoot" 0 0))
  (return _returnvalue))