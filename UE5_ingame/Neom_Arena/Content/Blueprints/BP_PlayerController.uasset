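; Player controller for click-to-move control of BP_Player, with a visible mouse cursor and clamped spring-arm zoom.
; Move input traces under the cursor, sets the Move state, shows a cursor marker and calls SimpleMoveToLocation.
; While held, a modulo timer and gate throttle repeat moves to once per interval.
; Tick returns the state to Idle on arrival or from any non-move state, and prints debug movement and hover data.
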(event Input|EnhancedActionEvents|EnhancedInputActionBomb
  (params (ActionValue :type Boolean) (ElapsedSeconds :type Float%20%28double-precision%29) (TriggeredSeconds :type Float%20%28double-precision%29) (InputAction :type Input%20Action%20Object%20Reference :default "/Game/Blueprints/PlayerInputActions/Bomb.Bomb")))

(event Input|EnhancedActionEvents|EnhancedInputActionMove
  (params (ActionValue :type Boolean) (ElapsedSeconds :type Float%20%28double-precision%29) (TriggeredSeconds :type Float%20%28double-precision%29) (InputAction :type Input%20Action%20Object%20Reference :default "/Game/Blueprints/PlayerInputActions/Move.Move")))

(event Input|EnhancedActionEvents|EnhancedInputActionMove
  (params (ActionValue :type Boolean) (ElapsedSeconds :type Float%20%28double-precision%29) (TriggeredSeconds :type Float%20%28double-precision%29) (InputAction :type Input%20Action%20Object%20Reference :default "/Game/Blueprints/PlayerInputActions/Move.Move"))
  (bind _rightclickinputinterval (Variables|Default|GetRightClickInputInterval))
  (:Triggered
    (Math|Float|CompareFloat (Math|Float|%(Float) ElapsedSeconds _rightclickinputinterval) (/ _rightclickinputinterval 2.0)
      (:>
        (Utilities|FlowControl|Gate false :!label _label
          (:Exit
            (CallFunction|ProcessMove)
            (goto _label Close))))
      (:<
        (goto _label Open))))
  (:Started
    (CallFunction|ProcessMove)))

(event Input|EnhancedActionEvents|EnhancedInputActionObjectSelect
  (params (ActionValue :type Boolean) (ElapsedSeconds :type Float%20%28double-precision%29) (TriggeredSeconds :type Float%20%28double-precision%29) (InputAction :type Input%20Action%20Object%20Reference :default "/Game/Blueprints/PlayerInputActions/ObjectSelect.ObjectSelect")))

(event Input|EnhancedActionEvents|EnhancedInputActionRuneSpell1
  (params (ActionValue :type Boolean) (ElapsedSeconds :type Float%20%28double-precision%29) (TriggeredSeconds :type Float%20%28double-precision%29) (InputAction :type Input%20Action%20Object%20Reference :default "/Game/Blueprints/PlayerInputActions/RuneSpell1.RuneSpell1")))

(event Input|EnhancedActionEvents|EnhancedInputActionRuneSpell2
  (params (ActionValue :type Boolean) (ElapsedSeconds :type Float%20%28double-precision%29) (TriggeredSeconds :type Float%20%28double-precision%29) (InputAction :type Input%20Action%20Object%20Reference :default "/Game/Blueprints/PlayerInputActions/RuneSpell2.RuneSpell2")))

(event Input|EnhancedActionEvents|EnhancedInputActionSkill1
  (params (ActionValue :type Boolean) (ElapsedSeconds :type Float%20%28double-precision%29) (TriggeredSeconds :type Float%20%28double-precision%29) (InputAction :type Input%20Action%20Object%20Reference :default "/Game/Blueprints/PlayerInputActions/Skill1.Skill1")))

(event Input|EnhancedActionEvents|EnhancedInputActionSkill2
  (params (ActionValue :type Boolean) (ElapsedSeconds :type Float%20%28double-precision%29) (TriggeredSeconds :type Float%20%28double-precision%29) (InputAction :type Input%20Action%20Object%20Reference :default "/Game/Blueprints/PlayerInputActions/Skill2.Skill2")))

(event Input|EnhancedActionEvents|EnhancedInputActionZoomINOut
  (params (ActionValue :type Float%20%28double-precision%29) (ElapsedSeconds :type Float%20%28double-precision%29) (TriggeredSeconds :type Float%20%28double-precision%29) (InputAction :type Input%20Action%20Object%20Reference :default "/Game/Blueprints/PlayerInputActions/ZoomINOut.ZoomINOut"))
  (bind _return (CallFunction|GetBPProject-D))
  (bind _myplayer (Variables|Default|GetMyPlayer))
  (bind _springarm (Variables|/Game/Characters/BP_Player.BP_Player_C|GetSpringArm _myplayer))
  (:Triggered
    (Variables|/Script/Engine.SpringArmComponent|SetTargetArmLength _springarm (Math|Float|Clamp(Float) (+ (Variables|/Script/Engine.SpringArmComponent|GetTargetArmLength _springarm) (* ActionValue -1e+02)) (Math|Conversions|ToFloat(Integer) (Variables|/Game/Blueprints/BP_Project-D.BP_Project-D_C|GetMinZoomSize _return)) (Math|Conversions|ToFloat(Integer) (Variables|/Game/Blueprints/BP_Project-D.BP_Project-D_C|GetMaxZoomSize _return))) :!label _label))
  (:Completed
    (goto _label)))

(event EventBeginPlay
  (bind _self self)
  (bind _returnvalue (PlayerController|LocalPlayerSubsystems|GetEnhancedInputLocalPlayerSubsystem _self))
  (bind _asbp_player (Utilities|Casting|CastToBP_Player (Pawn|GetControlledPawn)))
  (Variables|Default|SetMyPlayer _asbp_player)
  (Utilities|IsValid _returnvalue
    (:Is%20Valid
      (Input|AddMappingContext _returnvalue "/Game/Blueprints/PlayerInputActions/PlayerInputMapping.PlayerInputMapping" 0 "(bIgnoreAllPressedKeysUntilRelease=True,bForceImmediately=False)")
      (Variables|Default|SetOldDestination (Transformation|GetActorLocation (Variables|Default|GetMyPlayer)))
      (Variables|Default|SetbShowMouseCursor true)
      (Variables|Default|SetbEnableClickEvents true)
      (Variables|Default|SetbEnableMouseOverEvents true))))

(event EventTick
  (params (DeltaSeconds :type Float%20%28single-precision%29))
  (bind _actor (CallFunction|ObjectClicked?))
  (bind _olddestination (Variables|Default|GetOldDestination))
  (bind _myplayer (Variables|Default|GetMyPlayer))
  (bind _returnvalue (Transformation|GetActorLocation _myplayer))
  (bind _hitactor (Collision|BreakHitResult _actor))
  (CallFunction|UpdateInput)
  ;[1 1 1] Debug
  (CallFunction|AddDebugDataMapbyName 1 "State" (Utilities|String|EnumtoString (Variables|/Game/Characters/BP_Creature.BP_Creature_C|GetState (Variables|Default|GetMyPlayer))))
  (CallFunction|AddDebugDataMapbyName 2 "Dest" (Utilities|String|ToString(Vector2d) (Math|Vector2D|MakeVector2D (.x _olddestination) (.y _olddestination))))
  (CallFunction|AddDebugDataMapbyName 3 "Location" (Utilities|String|ToString(Vector2d) (Math|Vector2D|MakeVector2D (.x _returnvalue) (.y _returnvalue))))
  (CallFunction|SetDebugStringbyRow 4 (Utilities|String|ToString(Text) (Utilities|Text|FormatText "Difference between Dest and Location: {Diff}" (Math|Vector|VectorLength (Math|Vector|MakeVector (- (.x _returnvalue) (.x _olddestination)) (- (.y _returnvalue) (.y _olddestination)) 0.0)))) true)
  (CallFunction|SetDebugStringbyRow 5 (Utilities|String|ToString(Text) (Utilities|Text|FormatText "Velocity: {Vel}" (Math|Vector|VectorLength (Transformation|GetVelocity _myplayer)))) true)
  (bind _focusedself (Class|VBPClickable|OnFocused(Message) _hitactor))
  (Utilities|IsValid _focusedself
    (:Is%20Valid
      (CallFunction|AddDebugDataMapbyName 6 "Value" (Utilities|GetDisplayName _hitactor)))))

(fn ConstructionScript)

(fn UpdateInput
  (switch Utilities|FlowControl|Switch|SwitchonEstate (Variables|/Game/Characters/BP_Creature.BP_Creature_C|GetState (Variables|Default|GetMyPlayer))
    (:NewEnumerator0
      _)
    (:NewEnumerator1
      (if (CallFunction|IsArrived?)
        (Variables|/Game/Characters/BP_Creature.BP_Creature_C|SetState (Variables|Default|GetMyPlayer) "NewEnumerator0")))
    (:NewEnumerator13
      (Variables|/Game/Characters/BP_Creature.BP_Creature_C|SetState (Variables|Default|GetMyPlayer) "NewEnumerator0" :!label _label))
    (:NewEnumerator11
      (goto _label))
    (:NewEnumerator2
      (goto _label))
    (:NewEnumerator3
      (goto _label))
    (:NewEnumerator4
      (goto _label))
    (:NewEnumerator5
      (goto _label))
    (:NewEnumerator6
      (goto _label))
    (:NewEnumerator7
      (goto _label))
    (:NewEnumerator8
      (goto _label))
    (:NewEnumerator9
      (goto _label))
    (:NewEnumerator10
      (goto _label)))
  (if (CallFunction|IsKeyPressed?)
    _))

(fn UpdateMove
  (params (Destination :type Vector))
  (Variables|/Game/Characters/BP_Creature.BP_Creature_C|SetState (Variables|Default|GetMyPlayer) "NewEnumerator1")
  (CallFunction|MoveCursur (Game|GetGameMode) Destination "0, 0, 0")
  (AI|Navigation|SimpleMovetoLocation self Destination)
  (return Destination))

(fn IsArrived?
  (bind _olddestination (Variables|Default|GetOldDestination))
  (bind _myplayer (Variables|Default|GetMyPlayer))
  (bind _returnvalue (Transformation|GetActorLocation _myplayer))
  (return (<= (Math|Vector|VectorLength (- (Math|Vector|MakeVector (.x _olddestination) (.y _olddestination) 0.0) (Math|Vector|MakeVector (.x _returnvalue) (.y _returnvalue) 0.0))) 5.0)))

(fn IsMovingDirectionChanged?
  (params (Destination :type Vector))
  (if (Utilities|Operators|NotEqual(!=) Destination (Variables|Default|GetOldDestination) 0.0)
    (return true Destination)
    (else
      (return false "0, 0, 0"))))

(fn GetMouseHitLocation
  (return (.Location (Collision|BreakHitResult (.HitResult (Game|Player|GetHitResultUnderCursorbyChannel self "TraceTypeQuery1" true))))))

(fn IsKeyPressed?
  (return (Math|Boolean|ORBoolean (Input|EnhancedActionValues|GetSkill1) (Input|EnhancedActionValues|GetSkill2) (Input|EnhancedActionValues|GetSkill3) (Input|EnhancedActionValues|GetUltimateSkill) (Input|EnhancedActionValues|GetRuneSpell1) (Input|EnhancedActionValues|GetRuneSpell2) (Input|EnhancedActionValues|GetWard) (Input|EnhancedActionValues|GetBomb) (Input|EnhancedActionValues|GetObjectSelect) (Input|EnhancedActionValues|GetMove))))

(fn ProcessMove
  (bind _newdestination (CallFunction|UpdateMove (CallFunction|GetMouseHitLocation)))
  (Variables|Default|SetOldDestination _newdestination))

(fn ObjectClicked?
  (bind _array (Utilities|Array|MakeArray "ObjectTypeQuery2"))
  (bind _self self)
  (bind (_hitresult _returnvalue) (Class|PlayerController|GetHitResultUnderCursorforObjects _self _array true))
  (return _hitresult _returnvalue))