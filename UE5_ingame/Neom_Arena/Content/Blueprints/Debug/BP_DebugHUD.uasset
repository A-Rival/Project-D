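; BP_DebugHUD is a debug HUD that prints text lines over a backing rectangle on screen.
; It turns the HUD on at BeginPlay, then on each DrawHUD sizes the rectangle from the combined entry count.
; DebugStrings entries draw as "Key: Value" at their stored Row, while DabugDataString lines draw by array index from the top, so the two sets can overlap.
; Nothing in this file fills either collection.
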(event EventBeginPlay
  (Variables|Default|SetbShowHUD true))

(event EventDrawHUD
  (params (SizeX :type Integer) (SizeY :type Integer))
  (bind _dabugdatastring (Variables|Default|GetDabugDataString))
  (bind _debugstrings (Variables|Default|GetDebugStrings))
  (HUD|DrawRect "(R=0,G=0,B=0,A=1)" 0.0 0.0 3e+02 (Math|Conversions|ToFloat(Integer) (* (+ (Utilities|Array|Length (Variables|Default|GetDabugDataString)) (Utilities|Map|Length _debugstrings)) 11)))
  (bind _keys (Utilities|Map|Keys _debugstrings))
  (for _array_element _keys
    (HUD|DrawText (Utilities|String|ToString(Text) (Utilities|Text|FormatText "{Key}: {Value}" _array_element (.Value (Utilities|Struct|BreakDebugDataStructure (.Value (Utilities|Map|Find _debugstrings _array_element)))))) "(R=1.000000,G=1.000000,B=1.000000,A=1.000000)" 0.0 (Math|Conversions|ToFloat(Integer) (* (.Row (Utilities|Struct|BreakDebugDataStructure (.Value (Utilities|Map|Find _debugstrings _array_element)))) 10)) 0 1.0 false))
  (for _index (range 0 (- (Utilities|Array|Length _dabugdatastring) 1))
    (HUD|DrawText (Utilities|Array|Get(acopy) _dabugdatastring _index) "(R=1.000000,G=1.000000,B=1.000000,A=1.000000)" 0.0 (Math|Conversions|ToFloat(Integer) (* _index 10)) 0 1.0 false)))

(fn ConstructionScript)