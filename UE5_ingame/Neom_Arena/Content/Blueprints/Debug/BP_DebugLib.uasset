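; BP_DebugLib is a debug helper library that writes text and data to the BP_DebugHUD.
; GetDebugHud casts a player controller's HUD to BP_DebugHUD and returns a success flag, so both setters do nothing when it fails.
; Using player 0, one setter adds keyed row/value entries to the DebugStrings map, the other sets DabugDataString array entries by index.
; Both convert one-based row numbers to zero-based.
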(fn AddDebugDataMapbyName
  (params (Row :type Integer) (Key :type Name) (Value :type String))
  (bind (_hud _bsuccess) (CallFunction|GetDebugHud))
  (if _bsuccess
    (Utilities|Map|Add (Variables|/Game/Blueprints/Debug/BP_DebugHUD.BP_DebugHUD_C|GetDebugStrings _hud) Key (Utilities|Struct|MakeDebugDataStructure (- Row 1) Value))))

(fn SetDebugStringbyRow
  (params (Index :type Integer) (Text :type String) (bSizeToFit :type Boolean))
  (bind (_hud _bsuccess) (CallFunction|GetDebugHud))
  (if _bsuccess
    (Utilities|Array|SetArrayElem (Variables|/Game/Blueprints/Debug/BP_DebugHUD.BP_DebugHUD_C|GetDabugDataString _hud) (- Index 1) Text bSizeToFit)))

(fn GetDebugHud
  (params (PlayerIndex :type Integer))
  (bind _asbp_debug_hud (Utilities|Casting|CastToBP_DebugHUD (HUD|GetHUD (Game|GetPlayerController 0 PlayerIndex)))
    (:then
      (return _asbp_debug_hud true))
    (:CastFailed
      (return 0 false))))